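; Room trigger volume that tracks which FamilyMembers are inside and totals how long its linked Light stays on while the room is empty.
; An arriving member turns the light on; seated members stay counted when their overlap ends.
; An empty, lit room starts a timestamp and shows the box until someone enters or TurnOff runs, banking the elapsed time.
; Turning off an occupied room angers everyone inside.
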(event OnComponentBeginOverlap(Box)
  (params (OverlappedComponent :type Primitive%20Component%20Object%20Reference) (OtherActor :type Actor%20Object%20Reference) (OtherComp :type Primitive%20Component%20Object%20Reference) (OtherBodyIndex :type Integer) (bFromSweep :type Boolean) (SweepResult :type Hit%20Result%20Structure%20%28by%20ref%29))
  (bind _familiyin (Variables|Default|GetFamiliyIn))
  (bind _light (Variables|Default|GetLight))
  (bind _asfamily_member (Utilities|Casting|CastToFamilyMember OtherActor))
  (if (not (Utilities|Array|ContainsItem _familiyin _asfamily_member))
    (if (Variables|/Game/ScalaContent/Blueprints/EventManager/objects/Light.Light_C|GetState _light)
      _
      (else
        (Default|TurnON _light)))
    (Utilities|Array|Add _familiyin _asfamily_member)
    (if (> (Variables|Default|GetTimeout) 0.0)
      (Variables|Default|SetTotalTime (+ (- (Utilities|Time|GetTimeSeconds) (Variables|Default|GetTimeout)) (Variables|Default|GetTotalTime))))
    (Variables|Default|SetTimeout -1.0)
    (Development|SetHiddeninGame (Variables|Default|GetBox) true false)))

(event OnComponentEndOverlap(Box)
  (params (OverlappedComponent :type Primitive%20Component%20Object%20Reference) (OtherActor :type Actor%20Object%20Reference) (OtherComp :type Primitive%20Component%20Object%20Reference) (OtherBodyIndex :type Integer))
  (bind _familiyin (Variables|Default|GetFamiliyIn))
  (bind _asfamily_member (Utilities|Casting|CastToFamilyMember OtherActor))
  (if (not (Variables|/Game/ScalaContent/Blueprints/Characters/FamilyMember.FamilyMember_C|GetisSit _asfamily_member))
    (Utilities|Array|RemoveItem _familiyin _asfamily_member)
    (if (== (Utilities|Array|Length _familiyin) 0)
      (if (Variables|/Game/ScalaContent/Blueprints/EventManager/objects/Light.Light_C|GetState (Variables|Default|GetLight))
        (Variables|Default|SetTimeout (Utilities|Time|GetTimeSeconds))
        (Development|SetHiddeninGame (Variables|Default|GetBox) false false)))))

(event Custom|Turn%20on
  (if (== (Utilities|Array|Length (Variables|Default|GetFamiliyIn)) 0)
    (Variables|Default|SetTimeout (Utilities|Time|GetTimeSeconds))
    (Development|SetHiddeninGame (Variables|Default|GetBox) false false)))

(event Custom|Turn%20Off
  (bind _familiyin (Variables|Default|GetFamiliyIn))
  (if (== (Utilities|Array|Length _familiyin) 0)
    (if (> (Variables|Default|GetTimeout) 0.0)
      (Variables|Default|SetTotalTime (+ (- (Utilities|Time|GetTimeSeconds) (Variables|Default|GetTimeout)) (Variables|Default|GetTotalTime))))
    (Variables|Default|SetTimeout -1.0)
    (Development|SetHiddeninGame (Variables|Default|GetBox) true false)
    (else
      (Variables|Default|SetTimeout -1.0)
      (for _array_element _familiyin
        (Default|Angry _array_element))
      (Development|SetHiddeninGame (Variables|Default|GetBox) true false))))

(event EventBeginPlay
  (Variables|/Game/ScalaContent/Blueprints/EventManager/objects/Light.Light_C|SetRoomOverlap (Variables|Default|GetLight) self))

(fn ConstructionScript)