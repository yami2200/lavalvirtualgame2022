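; FamilyMember is an AI character for a family member who walks, sits, idles and gets angry, switching looping animations directly on the mesh.
; External callers drive it through Go, Sit, unSit, Idle and Angry, with Go, Sit and Idle reporting completion back through a passed-in Event object.
; Sit snaps it onto a seat with altered collision for a random time, and unSit restores its saved location.
; Angry also increments AngryTimes in GameInstanceLaval.
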(event Custom|Sit
  (params (Loc :type Vector) (Rot :type Rotator) (Event :type Event%20Object%20Reference))
  (bind (_x _y _z) (Math|Vector|BreakVector Loc))
  (bind _mesh (Variables|Character|GetMesh))
  (Components|Animation|PlayAnimation (Variables|Character|GetMesh) "/Game/ScalaContent/Char/Sitting__2__Anim_mixamo_com.Sitting__2__Anim_mixamo_com" true)
  (Variables|Default|SetisSit true)
  (Collision|SetCollisionEnabled (Variables|Collision|GetCapsuleComponent) "PhysicsOnly")
  (Variables|Default|SetoldRot (Transformation|GetWorldRotation _mesh))
  (Transformation|SetActorRotation Rot)
  (Transformation|SetWorldRotation _mesh (Math|Rotator|MakeRotator -5e+01 0.0 (- (.Yaw (Math|Rotator|BreakRotator Rot)) 9e+01)) false false)
  (Variables|Default|SetOldLoc (Transformation|GetActorLocation))
  (Transformation|SetActorLocation (Math|Vector|MakeVector _x _y (+ _z 7e+01)) false false)
  (Transformation|SetActorRotation Rot)
  (Utilities|FlowControl|Delay (Math|Random|RandomFloatinRange 8.0 2e+01))
  (Default|StopSitting Event)
  (Transformation|SetWorldRotation (Variables|Character|GetMesh) "0,-90.000000, 0" false false))

(event Custom|Go
  (params (Event :type Event%20Object%20Reference) (Location :type Vector))
  (AI|AIMoveTo self Location 0 5.0 false
    (:OnSuccess
      (Default|Arrived Event))
    (:OnFail
      (Default|Failed Event))))

(event Custom|unSit
  (Variables|Default|SetisSit false)
  (Collision|SetCollisionEnabled (Variables|Collision|GetCapsuleComponent) "QueryAndPhysics")
  (Transformation|SetActorLocation (Variables|Default|GetOldLoc) false false)
  (Components|Animation|PlayAnimation (Variables|Character|GetMesh) "/Game/ScalaContent/Char/Walking_Anim_mixamo_com.Walking_Anim_mixamo_com" true))

(event Custom|Idle
  (params (Event :type Event%20Object%20Reference))
  (Components|Animation|PlayAnimation (Variables|Character|GetMesh) "/Game/ScalaContent/Char/Walking_Anim_Unreal_Take.Walking_Anim_Unreal_Take" true)
  (Utilities|FlowControl|Delay (Math|Random|RandomFloatinRange 8.0 2e+01))
  (Components|Animation|PlayAnimation (Variables|Character|GetMesh) "/Game/ScalaContent/Char/Walking_Anim_mixamo_com.Walking_Anim_mixamo_com" true)
  (Default|StopIdle Event))

(event Custom|Angry
  (if (Variables|Default|GetisSit)
    (Transformation|SetWorldRotation (Variables|Character|GetMesh) "0,-90.000000, 0" false false))
  (Components|Animation|PlayAnimation (Variables|Character|GetMesh) "/Game/ScalaContent/Char/Angry__1__Anim_mixamo_com.Angry__1__Anim_mixamo_com" true)
  (bind _asgame_instance_laval (Utilities|Casting|CastToGameInstanceLaval (Game|GetGameInstance)))
  (Math|Integer|IncrementInt (Variables|/Game/ScalaContent/Blueprints/GameInstanceLaval.GameInstanceLaval_C|GetAngryTimes _asgame_instance_laval)))

(event EventBeginPlay
  (Components|Animation|PlayAnimation (Variables|Character|GetMesh) "/Game/ScalaContent/Char/Walking_Anim_mixamo_com.Walking_Anim_mixamo_com" true))

(fn ConstructionScript)