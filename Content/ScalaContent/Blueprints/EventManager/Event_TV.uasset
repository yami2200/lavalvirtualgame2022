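; Event Blueprint, used with the EventManager, in which a family member sits down to watch TV.
; On arrival, it seats the member at the transform supplied by SitRef, passes itself as the owning event and turns on the TV.
; When sitting stops, it tells the TV to stop watching, unseats the member and ends itself through the EventManager.
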(event EventArrived
  (bind (_location _rotation) (Default|GetTransformFamilyMember (Variables|Default|GetSitRef)))
  (Default|Sit (Variables|Default|GetFamilyMember) _location _rotation self)
  (CallFunction|Turnon (Variables|Default|GetTV)))

(event EventStopSitting
  (CallFunction|StopWatching (Variables|Default|GetTV))
  (Default|UnSit (Variables|Default|GetFamilyMember))
  (Default|EndEvent (Variables|Default|GetEventManager) self))