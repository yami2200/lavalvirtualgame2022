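; Event is a base object for a timed family-member activity run by the EventManager, carrying a FamilyMember and a Location.
; Start sends the FamilyMember toward the Location, and Arrived has it idle there.
; StopIdle tells the EventManager to end the event, while Failed reports the event and member as failed.
; StopSitting is an empty hook.
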(event Custom|Arrived
  (Default|Idle (Variables|Default|GetFamilyMember) self))

(event Custom|Failed
  (Default|FailedEvent (Variables|Default|GetEventManager) self (Variables|Default|GetFamilyMember)))

(event Custom|Start
  (Default|Go (Variables|Default|GetFamilyMember) self (Variables|Default|GetLocation)))

(event Custom|StopSitting)

(event Custom|StopIdle
  (Default|EndEvent (Variables|Default|GetEventManager) self))