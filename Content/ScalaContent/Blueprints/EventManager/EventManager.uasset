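; EventManager actor that hands out random events to every FamilyMember in the level.
; On BeginPlay it builds a pool of Event objects from placed sofa/TV, location, window and radiator lists, then starts one per member.
; Active events move to a used list; EndEvent assigns that member a new event before returning the finished one, avoiding immediate repeats.
; FailedEvent is an empty stub.
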(event Custom|New%20Event
  (params (Person :type Family%20Member%20Object%20Reference))
  (bind _events (Variables|Default|GetEvents))
  (bind _output_get (Variables|Default|SeteventTemp (Utilities|Array|Get(acopy) _events (Math|Random|RandomIntegerinRange 0 (- (Utilities|Array|Length _events) 1)))))
  (Variables|/Game/ScalaContent/Blueprints/EventManager/Event.Event_C|SetFamilyMember _output_get Person)
  (Utilities|Array|Add (Variables|Default|GetUsedEvents) _output_get)
  (Utilities|Array|RemoveItem _events _output_get)
  (Default|Start _output_get))

(event Custom|Generate%20Events
  (bind _self self)
  (bind _self_2 self)
  (for _array_element (Variables|Default|GetSofaTv)
    (bind _returnvalue (Game|ConstructObjectfromClass "/Game/ScalaContent/Blueprints/EventManager/Event_TV.Event_TV_C" self (.sofa _array_element) (.tv _array_element) (.room _array_element) (Transformation|GetActorLocation (.location _array_element)) 0 self))
    (Utilities|Array|Add (Variables|Default|GetEvents) _returnvalue))
  (for _array_element_2 (Variables|Default|GetListLocations)
    (bind _returnvalue_2 (Game|ConstructObjectfromClass "/Game/ScalaContent/Blueprints/EventManager/Event.Event_C" _self (.room _array_element_2) (Transformation|GetActorLocation (.pointeur _array_element_2)) 0 _self))
    (Utilities|Array|Add (Variables|Default|GetEvents) _returnvalue_2))
  (for _array_element_3 (Variables|Default|GetListWindows)
    (bind _returnvalue_3 (Game|ConstructObjectfromClass "/Game/ScalaContent/Blueprints/EventManager/Event_Window.Event_Window_C" _self_2 (.window (Utilities|Struct|BreakWindow _array_element_3)) "NewEnumerator0" (Transformation|GetActorLocation (.location (Utilities|Struct|BreakWindow _array_element_3))) 0 _self_2))
    (Utilities|Array|Add (Variables|Default|GetEvents) _returnvalue_3))
  (for _array_element_4 (Variables|Default|GetListRadiateurs)
    (bind _returnvalue_4 (Game|ConstructObjectfromClass "/Game/ScalaContent/Blueprints/EventManager/Event_Radiateur.Event_Radiateur_C" self (.rad (Utilities|Struct|BreakRadiateurStruct _array_element_4)) "NewEnumerator0" (Transformation|GetActorLocation (.location (Utilities|Struct|BreakRadiateurStruct _array_element_4))) 0 self))
    (Utilities|Array|Add (Variables|Default|GetEvents) _returnvalue_4)))

(event Custom|Failed%20Event
  (params (Event :type Event%20Object%20Reference) (Family%20Member :type Family%20Member%20Object%20Reference)))

(event Custom|EndEvent
  (params (Event :type Event%20Object%20Reference))
  (Utilities|Array|RemoveItem (Variables|Default|GetUsedEvents) Event)
  (CallFunction|NewEvent (Variables|/Game/ScalaContent/Blueprints/EventManager/Event.Event_C|GetFamilyMember Event))
  (Utilities|Array|Add (Variables|Default|GetEvents) Event))

(event EventBeginPlay
  (CallFunction|GenerateEvents)
  (bind _outactors (Actor|GetAllActorsOfClass "/Game/ScalaContent/Blueprints/Characters/FamilyMember.FamilyMember_C"))
  (bind _output_get (Variables|Default|SetlistFamily _outactors))
  (Utilities|FlowControl|Delay 0.0)
  (for _array_element _output_get
    (CallFunction|NewEvent _array_element)))

(fn ConstructionScript)