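; Radiator actor that toggles on and off with a particle effect and tracks how long it runs while a window is open.
; It starts off and registers itself with Windows, receiving open and close events that set its window flag.
; Heating with the window open starts a timestamp, and closing the window or switching off adds the elapsed time to a printed running total.
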(event Custom|Turn%20ON
  (Variables|Default|SetIsTurnedOn true)
  (Rendering|SetVisibility (Variables|Default|GetParticleSystem) true true)
  (if (Variables|Default|GetWinwodOpened)
    (Variables|Default|SetTimeout (Utilities|Time|GetTimeSeconds))))

(event Custom|Toggle
  (if (Variables|Default|GetIsTurnedOn)
    (CallFunction|TurnOFF)
    (else
      (CallFunction|TurnON))))

(event Custom|Turn%20OFF
  (Variables|Default|SetIsTurnedOn false)
  (Rendering|SetVisibility (Variables|Default|GetParticleSystem) false true)
  (CallFunction|AddTimeout))

(event Custom|Close%20Window
  (Variables|Default|SetWinwodOpened false)
  (if (Variables|Default|GetIsTurnedOn)
    (CallFunction|AddTimeout)))

(event Custom|Open%20Window
  (Variables|Default|SetWinwodOpened true)
  (if (Variables|Default|GetIsTurnedOn)
    (CallFunction|AddTimeout)
    (Variables|Default|SetTimeout (Utilities|Time|GetTimeSeconds))))

(event Custom|Add%20Timeout
  (if (> (Variables|Default|GetTimeout) 0.0)
    (bind _output_get (Variables|Default|SetTotalTime (+ (- (Utilities|Time|GetTimeSeconds) (Variables|Default|GetTimeout)) (Variables|Default|GetTotalTime))))
    (Development|PrintString (Utilities|String|ToString(Float) _output_get))
    (Variables|Default|SetTimeout -1.0)))

(event EventBeginPlay
  (CallFunction|TurnOFF)
  (Variables|/Game/ScalaContent/Blueprints/Windows/Window.Window_C|SetRadiateur (Variables|Default|Getwindows) self))

(fn ConstructionScript)